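; Clickable pickup actor that shows a dialog and removes itself once that dialog is done.
; Clicking creates a DialogWidget with the actor's Dialog text, adds it to the viewport and calls PickUpEvent with the widget reference.
; Tick polls the stored widget's Done flag and destroys the actor when it is set, without a validity check on the reference.
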(event `self.ReceiveActorOnClicked`
  (params (ButtonPressed :type "Key Structure"))
  (bind _returnvalue (`|CreateWidget` "/Game/Widgets/DialogWidget.DialogWidget_C"))
  (set `self.widgetRef` _returnvalue)
  (set `/Game/Widgets/DialogWidget.DialogText` (`self.Dialog`) _returnvalue)
  (`UserWidget.AddToViewport` _returnvalue 0)
  (`self.pickUp_event` (`self.widgetRef`)))

(event `self.ReceiveTick`
  (params (DeltaSeconds :type "Float (single-precision)"))
  (if (`/Game/Widgets/DialogWidget.done` (`self.widgetRef`))
    (`self.K2_DestroyActor`)))

(fn `UserConstructionScript`)
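; Jacket pickup that tells a door the coat has been collected.
; On BeginPlay it runs the parent logic, then binds its pickedUp event to the PickUpEvent dispatcher.
; When picked up, it prints a debug message, casts its Door reference to Door_Blueprint and sets that door's Coat flag to true.
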(event `self.ReceiveBeginPlay`
  (`parent.ReceiveBeginPlay`)
  (add `self.pickUp_event` (delegate `pickedUp`)))

(event `pickedUp`
  (`KismetSystemLibrary.PrintString` "I've been picked up")
  (bind _asdoor_blueprint (cast `/Game/bluePrints/Door_Blueprint` (`self.Door`)))
  (set `/Game/bluePrints/Door_Blueprint.coat` true _asdoor_blueprint))

(fn `UserConstructionScript`
  (`parent.UserConstructionScript`))
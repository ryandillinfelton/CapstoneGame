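; A clickable door Blueprint that moves the player to another level.
; On click it opens the configured level directly, except in Level2GB, where the Keys, Coat and File flags must all be set first.
; The first missing requirement shows its description through the Message function, which creates a DialogWidget with that text and adds it to the viewport.
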(event `self.ReceiveActorOnClicked`
  (params (ButtonPressed :type "Key Structure"))
  (`KismetSystemLibrary.PrintString` "door")
  (bind _returnvalue (`GameplayStatics.GetCurrentLevelName` true))
  (if (`KismetStringLibrary.EqualEqual_StrStr` _returnvalue "Level2GB")
    (if (`self.keys`)
      (if (`self.coat`)
        (if (`self.file`)
          (`KismetSystemLibrary.PrintString` "Leaving" :!label _label)
          (`GameplayStatics.OpenLevel` (`self.Level`))
          (else
            (`self.Message` (`self.FileDesc`))))
        (else
          (`self.Message` (`self.coatDesc`))))
      (else
        (`self.Message` (`self.keysDesc`))))
    (else
      (goto _label))))

(fn `Message`
  (params (MesgText :type Text))
  (returns (Widget :type "/Game/Widgets/DialogWidget Object Reference"))
  (bind _returnvalue (`|CreateWidget` "/Game/Widgets/DialogWidget.DialogWidget_C"))
  (set `/Game/Widgets/DialogWidget.DialogText` (`|MakeArray` MesgText) _returnvalue)
  (`UserWidget.AddToViewport` _returnvalue 0)
  (return _returnvalue))

(fn `UserConstructionScript`)
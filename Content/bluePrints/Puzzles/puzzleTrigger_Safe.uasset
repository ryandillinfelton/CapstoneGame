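; Clickable puzzle trigger actor for a safe with a three-digit combination.
; The first click shows a dialog widget with the first-click text and sets a flag.
; Each later click creates a safe widget, passing it the puzzle number, dialog lines, window reference and hardcoded solution code, then adds it to the viewport.
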(event `self.ReceiveActorOnClicked`
  (params (ButtonPressed :type "Key Structure"))
  (if (`self.ClickedOnce`)
    (bind _returnvalue (`|CreateWidget` "/Game/Widgets/SafeWidget.SafeWidget_C"))
    (set `/Game/Widgets/SafeWidget.PuzzleNumber` (`self.puzzleNumber`) _returnvalue)
    (set `/Game/Widgets/SafeWidget.DialogTextArray` (`self.Dialog`) _returnvalue)
    (set `/Game/Widgets/SafeWidget.Window` (`self.window`) _returnvalue)
    (set `/Game/Widgets/SafeWidget.SafeCodeSolution1` "8" _returnvalue)
    (set `/Game/Widgets/SafeWidget.SafeCodeSolution2` "6" _returnvalue)
    (set `/Game/Widgets/SafeWidget.SafeCodeSolution3` "5" _returnvalue)
    (`UserWidget.AddToViewport` _returnvalue 0)
    (else
      ;[1 1 1] on first click
      (bind _returnvalue_2 (`|CreateWidget` "/Game/Widgets/DialogWidget.DialogWidget_C"))
      (set `/Game/Widgets/DialogWidget.DialogText` (`|MakeArray` (`self.FirstClickText`)) _returnvalue_2)
      (`UserWidget.AddToViewport` _returnvalue_2 0)
      (set `self.ClickedOnce` true))))

(fn `UserConstructionScript`)
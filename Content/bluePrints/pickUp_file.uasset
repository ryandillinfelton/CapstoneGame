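; A pickup actor for a file that, when collected, sets the File flag on its linked Door_Blueprint.
; BeginPlay binds the parent's PickUpEvent to a handler that stores the description widget and updates the door.
; Tick polls that widget's dialog number and, on the second line, adds a FolderWidget to the viewport with the dialog as parent.
; The check has no one-shot guard, so it creates a new widget every frame that line remains current.
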(event `self.ReceiveBeginPlay`
  (`parent.ReceiveBeginPlay`)
  (add `self.pickUp_event` (delegate `pickedUp`)))

(event `pickedUp` :!signature `self.pickUp_event`
  (params (DescWidget :type "/Game/Widgets/DialogWidget Object Reference"))
  (set `self.DescWidget` DescWidget)
  (bind _asdoor_blueprint (cast `/Game/bluePrints/Door_Blueprint` (`self.Door`)))
  (set `/Game/bluePrints/Door_Blueprint.file` true _asdoor_blueprint))

(event `self.ReceiveTick`
  (params (DeltaSeconds :type "Float (single-precision)"))
  (bind _descwidget (`self.DescWidget`))
  ;[1 1 1] if on the second line of dialog
  (`parent.ReceiveTick` DeltaSeconds)
  (if (== (`/Game/Widgets/DialogWidget.dialogNumber` _descwidget) 1)
    (bind _returnvalue (`|CreateWidget` "/Game/Widgets/FolderWidget.FolderWidget_C"))
    (set `/Game/Widgets/FolderWidget.parentDialogWidget` _descwidget _returnvalue)
    (`UserWidget.AddToViewport` _returnvalue 1)))

(fn `UserConstructionScript`
  (`parent.UserConstructionScript`))